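; Skeleton character that wanders back and forth along the spline of a referenced path actor, pausing at random.
; Tick steps its distance along the spline by a fixed per-frame amount, wrapping at both ends, and offsets rotation to face the travel direction.
; A self-rescheduling random timer alternates CurrentState between a pause and a randomly chosen forward or backward walk.
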(event Custom|MoveLogicLoop
  (if (== (Math|Integer|%(Integer) (Variables|Default|GetCurrentState) 2) 0)
    (Variables|Default|SetCurrentState 1)
    (else
      (Variables|Default|SetCurrentState (Math|Integer|SelectInt 0 2 (Math|Random|RandomBool)))))
  (Utilities|Time|SetTimerbyEvent (delegate Custom|MoveLogicLoop) (Math|Random|RandomFloatinRange 2.0 5.0)))

(event EventBeginPlay
  (CallFunction|MoveLogicLoop)
  (if (Utilities|IsValid (Variables|Default|GetPathRef))
    (Utilities|Time|SetTimerbyEvent (delegate Custom|MoveLogicLoop) (Math|Random|RandomFloatinRange 2.0 5.0))))

(event Collision|EventActorBeginOverlap
  (params (OtherActor :type Actor%20Object%20Reference)))

(event EventTick
  (params (DeltaSeconds :type Float%20%28single-precision%29))
  (bind _pathref (Variables|Default|GetPathRef))
  (bind _pathref_2 (Variables|Default|GetPathRef))
  (bind _spline (Variables|/Game/Characters/Sangsang/BP_PatrolPath.BP_PatrolPath_C|GetSpline _pathref))
  (bind _spline_2 (Variables|/Game/Characters/Sangsang/BP_PatrolPath.BP_PatrolPath_C|GetSpline _pathref_2))
  (bind _returnvalue (Spline|GetSplineLength _spline))
  (switch int (Variables|Default|GetCurrentState)
    (:0
      (Variables|Default|SetDistanceOnPath (|(((Distance%Length)+Length)%Length) (+ (Variables|Default|GetDistanceOnPath) 0.5) _returnvalue))
      (Transformation|SetActorLocationAndRotation (Spline|GetLocationatDistanceAlongSpline _spline_2 (Variables|Default|GetDistanceOnPath) "World") (Math|Rotator|CombineRotators (Spline|GetRotationatDistanceAlongSpline _spline_2 (Variables|Default|GetDistanceOnPath) "World") (Utilities|Select :Index (Variables|Default|GetCurrentState) :Option%200 "0.000000,-90.000000,0.000000" :Option%201 "0.000000,-90.000000,0.000000" :Option%202 "0.000000,90.000000,0.000000" :Option%203 "0.000000,90.000000,0.000000")) :!label _label))
    (:1
      (Transformation|SetActorLocationAndRotation (Spline|GetLocationatDistanceAlongSpline _spline_2 (Variables|Default|GetDistanceOnPath) "World") (Transformation|GetActorRotation) :!label _label_2))
    (:2
      (Variables|Default|SetDistanceOnPath (|(((Distance%Length)+Length)%Length) (- (Variables|Default|GetDistanceOnPath) 0.5) _returnvalue))
      (goto _label))
    (:3
      (goto _label_2))))

(fn ConstructionScript)
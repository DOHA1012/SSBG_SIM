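; BP_Camera is a camera actor that follows a target actor at an offset and can switch to a fixed high position.
; Tick places it at the target's location plus CameraOffset while IsTracking is set.
; CameraMove stops tracking and lerps it along a timeline to a fixed world point.
; CameraMove_Reverse resumes tracking immediately, blending the offset from the current relative position to the follow offset, so the return follows a moving target.
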(event Custom|CameraMove
  (Variables|Default|SetbIsTracking false)
  (Variables|Default|SetStartLocation (Transformation|GetActorLocation))
  (bind _alpha (Timeline|타임라인 PlayFromStart)
    (:Update
      (Transformation|SetActorLocation (Math|Vector|Lerp(Vector) (Variables|Default|GetStartLocation) "0.000000,0.000000,2570.000000" _alpha) false false))))

(event Custom|CameraMove_Reverse
  (bind _output_get (Variables|Default|SetStartLocation (- (Transformation|GetActorLocation) (Transformation|GetActorLocation (Variables|Default|GetTargetActor)))))
  (Variables|Default|SetCameraOffset _output_get)
  (Variables|Default|SetbIsTracking true)
  (bind _alpha (Timeline|타임라인_1 PlayFromStart)
    (:Update
      (Variables|Default|SetCameraOffset (Math|Vector|Lerp(Vector) (Variables|Default|GetStartLocation) "-920.000000,0.000000,642.000000" _alpha)))))

(event EventBeginPlay)

(event Collision|EventActorBeginOverlap
  (params (OtherActor :type Actor%20Object%20Reference)))

(event EventTick
  (params (DeltaSeconds :type Float%20%28single-precision%29))
  (if (Variables|Default|GetbIsTracking)
    (Transformation|SetActorLocation (+ (Transformation|GetActorLocation (Variables|Default|GetTargetActor)) (Variables|Default|GetCameraOffset)) false false)))

(fn ConstructionScript)
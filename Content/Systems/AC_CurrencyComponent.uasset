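; Actor component that tracks the player's academic, extra and idle currencies, experience and level.
; A looping timer grants idle currency each minute, and item boosts scale all currency gains.
; Weather-scaled experience feeds a recursive level-up check against DT_LevelEXP.
; Saving passes truncated currencies and experience, but not level, to ApplyAndCache; the update-from-server assignments are unwired.
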(event Custom|OnMinuteUpdate
  (CallFunction|AddCurrency 1.0 "NewEnumerator2"))

(event EventBeginPlay
  (Utilities|Time|SetTimerbyEvent (delegate Custom|OnMinuteUpdate) 6e+01 true))

(fn CheckLevelUp
  (bind _returnvalue (Utilities|GetDataTableRow "/Game/Data/DT_LevelEXP.DT_LevelEXP" (Utilities|String|StringToName (Utilities|String|ToString(Integer) (Variables|Default|GetUserLevel))))
    (:then
      (if (>= (Variables|Default|GetCurrentExp) (.RequiredEXP (Utilities|Struct|BreakS_LevelData _returnvalue)))
        (Variables|Default|SetUserLevel (+ (Variables|Default|GetUserLevel) 1))
        (Variables|Default|SetCurrentExp (- (Variables|Default|GetCurrentExp) (.RequiredEXP (Utilities|Struct|BreakS_LevelData _returnvalue))))
        (CallFunction|CheckLevelUp)))))

(fn AddExperience
  (params (Amount :type Float%20%28double-precision%29))
  (Variables|Default|SetCurrentExp (+ (Variables|Default|GetCurrentExp) (* Amount (Variables|Default|GetWeatherMultiplier))))
  (CallFunction|CheckLevelUp))

(fn UpdateWeatherMultiplier
  (switch Utilities|FlowControl|Switch|SwitchonE_WeatherState (Variables|Default|GetCurrentWeather)
    (:NewEnumerator0
      (Variables|Default|SetWeatherMultiplier 1.2))
    (:NewEnumerator1
      (Variables|Default|SetWeatherMultiplier 1.0))
    (:NewEnumerator2
      (Variables|Default|SetWeatherMultiplier 0.8))
    (:NewEnumerator3
      (Variables|Default|SetWeatherMultiplier 0.8))))

(fn AddCurrency
  (params (Amount :type Float%20%28double-precision%29) (CurrencyType :type E_CurrencyType%20Enum :default "NewEnumerator0"))
  (switch Utilities|FlowControl|Switch|SwitchonE_CurrencyType CurrencyType
    (:NewEnumerator0
      (Variables|Default|SetAcademicCurrency (+ (* Amount (Variables|Default|GetAcademicItemBoost)) (Variables|Default|GetAcademicCurrency))))
    (:NewEnumerator1
      (Variables|Default|SetExtraCurrency (+ (* Amount (Variables|Default|GetExtraItemBoost)) (Variables|Default|GetExtraCurrency))))
    (:NewEnumerator2
      (Variables|Default|SetIdleCurrency (+ (Variables|Default|GetIdleCurrency) (* Amount (Variables|Default|GetIdleItemBoost)))))))

(fn UpdateCurrencyfromServer
  (params (NewAcademic :type Float%20%28double-precision%29) (NewExtra :type Float%20%28double-precision%29) (NewIdle :type Float%20%28double-precision%29)))

(fn RequestSavetoServer
  (Class|EclassAPIHandler|ApplyandCache (Utilities|Struct|MakeEclassData (Math|Float|Truncate (Variables|Default|GetAcademicCurrency)) (Math|Float|Truncate (Variables|Default|GetExtraCurrency)) (Math|Float|Truncate (Variables|Default|GetIdleCurrency)) (Math|Float|Truncate (Variables|Default|GetCurrentExp)))))
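; Time manager component that fires a daily reset event on a 6:00 Korea Standard Time boundary.
; BeginPlay requests server time, and ProcessServerTime converts a UTC time to KST at hour precision.
; CheckForReset shifts current and last reset times back six hours, compares only their day-of-month, and broadcasts OnDailyReset when the current day is greater, then stores the new reset time.
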(event EventBeginPlay
  (Class|EclassAPIHandler|GetServerTime (EventDispatchers|CreateEvent :!event ProcessServerTime)))

(fn CheckforReset
  (params (CurrentKST :type Date%20Time%20Structure))
  (if (> (.Day (Math|DateTime|BreakDateTime (- CurrentKST (Math|Timespan|MakeTimespan 0 6)))) (.Day (Math|DateTime|BreakDateTime (- (Variables|Default|GetLastResetTime) (Math|Timespan|MakeTimespan 0 6)))))
    (Default|CallOnDailyReset)
    (Variables|Default|SetLastResetTime CurrentKST)
    (return)
    (else
      (return))))

(fn ProcessServerTime
  (params (ServerTime :type Server%20Time%20Structure))
  (bind (_utchour _utcday _utcmonth _utcyear) (Utilities|Struct|BreakServerTime ServerTime))
  (CallFunction|CheckforReset (+ (Math|DateTime|MakeDateTime _utcyear _utcmonth _utcday _utchour) (Math|Timespan|MakeTimespan 0 9))))